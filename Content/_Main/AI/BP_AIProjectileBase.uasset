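; Base AI projectile that damages living players on overlap and passes through actors tagged Enemy.
; On Body overlap, the server applies damage to living Player-tagged actors, crediting the projectile's owner.
; Those hits and hits on other non-enemy actors play particle and sound through Multi_PlayHitVFX, then destroy the projectile after a short delay.
; A leftover debug "Hello" print fires on every overlap.
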(event `self.Body.OnComponentBeginOverlap`
  (params (OverlappedComponent :type "PrimitiveComponent Object Reference") (OtherActor :type "Actor Object Reference") (OtherComp :type "PrimitiveComponent Object Reference") (OtherBodyIndex :type Integer) (bFromSweep :type Boolean) (SweepResult :type "HitResult Structure (by ref)"))
  (bind (_bblockinghit _binitialoverlap _time _distance _location) (`GameplayStatics.BreakHitResult` SweepResult))
  (`KismetSystemLibrary.PrintString` "Hello")
  (`/Engine/EditorBlueprintResources/ActorMacros.Switch Has Authority`
    (:`Authority`
      (if (`self.ActorHasTag` OtherActor "Player")
        (bind _state (message `/Game/_Main/Interfaces/IBP_PlayerCharacter.PlayerAliveState` OtherActor))
        (if _state
          (set `self.Other Actor` OtherActor)
          (bind _output_get (set `self.HitLocation` _location))
          (`self.Multi_PlayHitVFX` (`self.HitParticle`) _output_get (`self.HitScale`) (`self.HitSound`))
          (`GameplayStatics.ApplyDamage` OtherActor (`self.Damage`) null (`self.GetOwner`) "/Script/Engine.DamageType")
          (`KismetSystemLibrary.Delay` 0.1 :!label _label)
          (`self.K2_DestroyActor`))
        (elif (not (`self.ActorHasTag` OtherActor "Enemy"))
          (`self.Multi_PlayHitVFX` (`self.HitParticle`) _location (`self.HitScale`) (`self.HitSound`))
          (goto _label))))))

(event `Multi_PlayHitVFX`
  (params (EmitterTemplate :type "ParticleSystem Object Reference") (Location :type "Vector Structure") (Scale :type "Vector Structure") (Sound :type "SoundBase Object Reference"))
  (`GameplayStatics.SpawnEmitterAtLocation` EmitterTemplate Location (struct) Scale)
  (`GameplayStatics.PlaySoundAtLocation` Sound Location (struct) 1.0 1.0 0.0 null null null))

(fn `UserConstructionScript`)