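; Player controller that drives its possessed pawn's movement from the MoveForward and MoveRight axis inputs.
; It caches the controlled pawn on BeginPlay and adds movement input along the forward and right vectors of the pawn's control rotation.
; Movement is applied only while the pawn is valid and the MovAvailable flag is true, which the MovementeAvailable event sets to enable or block movement.
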(event `self.ReceiveBeginPlay`
  (set `self.ControlledPawn` (`self.K2_GetPawn`)))

(event `InputAxis|MoveForward`
  (params (AxisValue :type "Float (single-precision)"))
  (bind _controlledpawn (`self.ControlledPawn`))
  (`self.ControlledPawn`
    (:`then`
      (if (`self.bMovAvailable`)
        (`Pawn.AddMovementInput` _controlledpawn (`KismetMathLibrary.GetForwardVector` (`Pawn.GetControlRotation` _controlledpawn)) AxisValue false)))
    (:`else`)))

(event `InputAxis|MoveRight`
  (params (AxisValue :type "Float (single-precision)"))
  (bind _controlledpawn (`self.ControlledPawn`))
  (`self.ControlledPawn`
    (:`then`
      (if (`self.bMovAvailable`)
        (`Pawn.AddMovementInput` _controlledpawn (`KismetMathLibrary.GetRightVector` (`Pawn.GetControlRotation` _controlledpawn)) AxisValue false)))
    (:`else`)))

(event `/Game/_Main/Interfaces/IBP_PlayerController.MovementeAvailable`
  (params (State :type Boolean))
  (set `self.bMovAvailable` State))

(fn `UserConstructionScript`)