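; Base character Blueprint providing shared attack playback and spawn-location tracking, apparently for AI as well.
; After a one-second delay on BeginPlay it caches its controller and location, and AISpawnedLocation can re-record that location for the getter.
; Multi-prefixed events play an attack montage, with its sound fired on Notify Begin at the actor's location, and standalone hit sounds.
; A helper picks a random montage section from AttackSection for attack variety.
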(event `self.ReceiveBeginPlay`
  (`KismetSystemLibrary.Delay` 1.0)
  (set `self.ControllerRef` (`self.GetController`))
  (set `self.SpawnLocation` (`self.K2_GetActorLocation`)))

(event `AISpawnedLocation`
  (set `self.SpawnLocation` (`self.K2_GetActorLocation`)))

(event `Multi_PrimeAttack`
  (params (InSkeletalMeshComponent :type "SkeletalMeshComponent Object Reference") (MontageToPlay :type "AnimMontage Object Reference") (Sound :type "SoundBase Object Reference") (StartingSection :type Name))
  (`|PlayMontage` InSkeletalMeshComponent MontageToPlay 1.0 0.0 StartingSection
    (:`OnNotifyBegin`
      (`GameplayStatics.PlaySoundAtLocation` Sound (`self.K2_GetActorLocation`) (struct) 1.0 1.0 0.0 null null null))))

(event `Multi_PlayHitSound`
  (params (Sound :type "SoundBase Object Reference") (Location :type "Vector Structure"))
  (`GameplayStatics.PlaySoundAtLocation` Sound Location (struct) 1.0 1.0 0.0 null null null))

(fn `fGetMontageSection`
  (returns (Section :type Name))
  (bind _attacksection (`self.AttackSection`))
  (return (`|GetArrayItem` _attacksection (`KismetMathLibrary.RandomIntegerInRange` 0 (- (`KismetArrayLibrary.Array_Length` _attacksection) 1)))))

(fn `fGetSpawnedLocation`
  (returns (spawnedLocation :type "Vector Structure"))
  (return (`self.SpawnLocation`)))

(fn `UserConstructionScript`)