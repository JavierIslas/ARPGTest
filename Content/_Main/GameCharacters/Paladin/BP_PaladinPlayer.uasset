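; Paladin player character Blueprint that adds a melee attack and damage handling on top of its parent class.
; The server-side primary attack briefly locks attacking, notifies the controller about movement availability and multicasts a montage section with sound.
; A collision-toggled hitbox applies authority-only damage to Enemy-tagged actors, with a DoOnce limiting the multicast hit sound until the attack resets it.
; Incoming damage reduces health in the stats struct and triggers the server kill at zero.
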(event `self.server_PrimeAttack`
  (set `self.bCanAttack` false)
  (message `/Game/_Main/Interfaces/IBP_PlayerController.MovementeAvailable` (`self.ControllerRef`) false)
  (`self.Multi_PrimeAttack` (`self.Mesh`) (`self.AttackMontage`) (`self.AttackSound`) (`self.fGetMontageSection`))
  (`KismetSystemLibrary.Delay` 0.4)
  (message `/Game/_Main/Interfaces/IBP_PlayerController.MovementeAvailable` (`self.ControllerRef`) true)
  (set `self.bCanAttack` true)
  (`self.ResetMeleeSound`))

(event `self.MeleeHitBox.OnComponentBeginOverlap`
  (params (OverlappedComponent :type "PrimitiveComponent Object Reference") (OtherActor :type "Actor Object Reference") (OtherComp :type "PrimitiveComponent Object Reference") (OtherBodyIndex :type Integer) (bFromSweep :type Boolean) (SweepResult :type "HitResult Structure (by ref)"))
  (`/Engine/EditorBlueprintResources/ActorMacros.Switch Has Authority`
    (:`Authority`
      (if (`self.ActorHasTag` OtherActor "Enemy")
        (`GameplayStatics.ApplyDamage` OtherActor 10.0 (`self.ControllerRef`) self "/Script/Engine.DamageType")
        (`/Engine/EditorBlueprintResources/StandardMacros.DoOnce` false :!label _label
          (:`Completed`
            (`self.Multi_PlayHitSound` null (`self.K2_GetActorLocation`))))))))

(event `ResetMeleeSound`
  (goto _label :!via `Reset`))

(event `/Game/_Main/Interfaces/IBP_PlayerCharacter.SetAttackColl`
  (params (collision :type "ECollisionEnabled Enum" :default "NoCollision"))
  (`PrimitiveComponent.SetCollisionEnabled` (`self.MeleeHitBox`) collision))

(event `self.ReceiveAnyDamage`
  (params (Damage :type "Float (single-precision)") (DamageType :type "DamageType Object Reference") (InstigatedBy :type "Controller Object Reference") (DamageCauser :type "Actor Object Reference"))
  (bind _stats (`self.Stats`))
  (bind _structout (setmembers `/Game/_Main/GameLogic/S_Statistics` :`StructRef` _stats :`currentHealt` (- (`.currentHealt_2_95A1062B44B529AE03B05F9762DE08E3` (break `/Game/_Main/GameLogic/S_Statistics` _stats)) Damage)))
  (if (<= (`.currentHealt_2_95A1062B44B529AE03B05F9762DE08E3` (break `/Game/_Main/GameLogic/S_Statistics` _structout)) 0.0)
    (`self.Server_KillPlayer`)))

(fn `UserConstructionScript`
  (`parent.UserConstructionScript`))