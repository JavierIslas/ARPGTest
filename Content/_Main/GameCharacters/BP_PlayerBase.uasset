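; Base player character for a networked game with lives, handling attack input, death and respawn.
; Attack input calls a server event when the player is alive and able to attack; that event and AnyDamage are empty here.
; Server kill clears Alive, multicasts death to the AnimInstance and messages the controller about movement.
; After a delay, it has the controller decrease lives and respawn the same class, then destroys this actor.
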(event `InputAction|PrimeAttack`
  (params (Key :type "Key Structure"))
  (:`Pressed`
    (bind _valid (`self.canAttack`))
    (if _valid
      (`self.server_PrimeAttack`))))

(event `server_PrimeAttack`)

(event `self.ReceiveAnyDamage`
  (params (Damage :type "Float (single-precision)") (DamageType :type "DamageType Object Reference") (InstigatedBy :type "Controller Object Reference") (DamageCauser :type "Actor Object Reference")))

(event `Server_KillPlayer`
  (if (`self.bAlive`)
    (set `self.bAlive` false)
    (`self.Multi_PlayerDead`)
    (message `/Game/_Main/Interfaces/IBP_PlayerController.MovementeAvailable` (`self.ControllerRef`) false)
    (`KismetSystemLibrary.Delay` 3.0)
    (`self.Server_RespawnPlayer`)))

(event `Multi_PlayerDead`
  (message `/Game/_Main/Interfaces/IBP_AnimBP.SetDead` (`SkeletalMeshComponent.GetAnimInstance` (`self.Mesh`))))

(event `Server_RespawnPlayer`
  (bind _controllerref (`self.ControllerRef`))
  (message `/Game/_Main/Interfaces/IBP_PlayerController.DecreaseLives` _controllerref)
  (message `/Game/_Main/Interfaces/IBP_PlayerController.PlayerRespawn` _controllerref (`self.Class`) (`self.SpawnLocation`))
  (`KismetSystemLibrary.Delay` 5.0)
  (`self.K2_DestroyActor`))

(fn `canAttack`
  (returns (valid :type Boolean))
  (if (`self.bAlive`)
    (if (`self.bCanAttack`)
      (return true)
      (else
        _)))
  (return false))

(fn `PlayerAliveState`
  (returns (State :type Boolean))
  (return (`self.bAlive`)))

(fn `UserConstructionScript`)